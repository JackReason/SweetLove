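; BP_Candy is the pool objective whose loss ends the game, passing through water, dome and candy stages.
; Damage lowers the water and updates the HUD bar; draining resets health for the dome, whose break removes the pedestal and exposes the candy to defeat.
; A looping timeline orbits a target point via sine/cosine, and a one-second timer reports its location to BP_WaveManager, pausing during the drain transition.
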(event `self.ReceiveBeginPlay`
  ;[1 1 1] Needed for targeting math
  (set `self.TargetOriginalLenth` (`KismetMathLibrary.VSizeXY` (`SceneComponent.RelativeLocation` (`self.Scene`))))
  ;[1 1 1] for the manager
  (`self.StartMovingTarget`)
  (bind _returnvalue (`KismetSystemLibrary.K2_SetTimer` null "SendInfoToManager" 1.0 true))
  (set `self.InfoToManager_Handle` _returnvalue))

(event `self.ReceiveAnyDamage`
  (params (Damage :type "Float (single-precision)") (DamageType :type "DamageType Object Reference") (InstigatedBy :type "Controller Object Reference") (DamageCauser :type "Actor Object Reference"))
  ;[1 1 1] Main Flow / Take damage
  (bind _output_get (set `self.Health` (- (`self.Health`) (/ Damage 3.0))))
  (if (`self.WaterMode`)
    (`SceneComponent.K2_SetRelativeLocation` (`self.Water`) (`KismetMathLibrary.MakeVector` 0.0 0.0 (`KismetMathLibrary.MapRangeClamped` _output_get 100.0 0.0 45.0 -250.0)) false false)
    (`self.HUDInfo`)
    (else
      (`self.HUDInfo`)))
  (if (<= (`self.Health`) 0.0)
    (if (`self.WaterMode`)
      (`self.PoolIsEmpty_Event`)
      (elif (`self.DomeMode`)
        (`self.DomeIsBroken`)
        (elif (`self.CandyMode`)
          (message `/Game/SweetLove/Interfaces/BPi_GameOverCall.GameOver` (`GameplayStatics.GetGameMode`) false))))))

(event `PoolIsEmpty_Event`
  ;[1 1 1] End Of the first stage
  (`KismetSystemLibrary.K2_PauseTimerHandle` (`self.InfoToManager_Handle`))
  (`PrimitiveComponent.SetMaterial` (`self.Water`) 0 "/Engine/EngineMaterials/WorldGridMaterial.WorldGridMaterial")
  (bind (_direction _zkoef) (`Timeline|Timeline` :!via `PlayFromStart`)
    (:`Update`
      (`SceneComponent.K2_SetRelativeLocation` (`self.Water`) (`KismetMathLibrary.MakeVector` 0.0 0.0 (+ (`self.LowestPointZ`) (* (`self.Z`) _zkoef))) false false))
    (:`Finished`
      (`self.AjustPool_Event`)
      (`self.HUDInfo`))))

(event `AjustPool_Event`
  ;[1 1 1] Ajusting pool for the second stage
  (set `self.WaterMode` false)
  (`self.StopMovingTarget`)
  (`SceneComponent.K2_SetRelativeLocation` (`self.Scene`) (0.0 240.0 260.0) false false)
  (set `self.TargetOriginalLenth` (`KismetMathLibrary.VSizeXY` (`SceneComponent.RelativeLocation` (`self.Scene`))))
  (`KismetSystemLibrary.K2_UnPauseTimerHandle` (`self.InfoToManager_Handle`))
  (`self.StartMovingTarget`)
  (`SceneComponent.SetRelativeScale3D` (`self.Sphere`) (126.0 116.0 11.0))
  (set `self.Health` 100.0)
  (set `self.DomeMode` true))

(event `DomeIsBroken`
  ;[1 1 1] End od the second phase / start of the final
  (`ActorComponent.K2_DestroyComponent` (`self.SM_Pedestal`))
  (set `self.DomeMode` false)
  (set `self.CandyMode` true))

(event `StartMovingTarget`
  ;[1 1 1] Creating Target for the Manager
  (bind (_direction _newtrack_0) (`Timeline|MovingTarget` :!via `PlayFromStart` :!label _label)
    (:`Update`
      (`self.Move Target` _newtrack_0))
    (:`Finished`
      (`self.StartMovingTarget`))))

(event `StopMovingTarget`
  ;[1 1 1] Creating Target for the Manager
  (goto _label :!via `Stop`))

(fn `HUDInfo`
  (locals (WaterText :type Text :default "NSLOCTEXT(\"\", \"89ED51BF41C9C80AFD73FC881DD8EE20\", \"Water Level\")") (DomeText :type Text :default "NSLOCTEXT(\"\", \"41404C90462E8FE52EED5D9C452A21C2\", \"Dome Resilience\")"))
  (bind _returnvalue (`KismetMathLibrary.MapRangeClamped` (`self.Health`) 0.0 100.0 0.0 1.0))
  (bind _asbp_hud (cast `/Game/SweetLove/GameBluePrints/BP_HUD` (`PlayerController.GetHUD` (`GameplayStatics.GetPlayerController` 0))))
  (if (`self.WaterMode`)
    (`/Game/SweetLove/GameBluePrints/BP_HUD.ChangePoolBar` _asbp_hud _returnvalue (`local.WaterText`))
    (else
      (`/Game/SweetLove/GameBluePrints/BP_HUD.ChangePoolBar` _asbp_hud _returnvalue (`local.DomeText`)))))

(fn `Move Target`
  (params (Angle :type "Float (double-precision)"))
  (bind _targetoriginallenth (`self.TargetOriginalLenth`))
  (`SceneComponent.K2_SetRelativeLocation` (`self.Scene`) (`KismetMathLibrary.MakeVector` (* _targetoriginallenth (`KismetMathLibrary.DegSin` Angle)) (* _targetoriginallenth (`KismetMathLibrary.DegCos` Angle)) 260.0) false false))

(fn `SendInfoToManager`
  (bind _returnvalue (`GameplayStatics.GetActorOfClass` "/Game/SweetLove/Enemies/EvilManager/BP_WaveManager.BP_WaveManager_C"))
  (`/Engine/EditorBlueprintResources/StandardMacros.IsValid` _returnvalue
    (:`Is Valid`
      (message `/Game/SweetLove/Interfaces/BPi_RecieveTargetInfo.RecieveInfo` _returnvalue (`SceneComponent.K2_GetComponentLocation` (`self.Scene`))))))

(fn `UserConstructionScript`)