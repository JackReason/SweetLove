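; BP_SnowThrower is a spinning weapon that launches snow or ice projectiles.
; Looping timers ramp the RotatingMovement rate up to a cap or down toward zero.
; Overlaps on two spatula components spawn the selected projectile at the root, yawed 90 degrees, if that ammo remains.
; Each ammo type has its own reserve, filled at BeginPlay and drained per shot, and ChangeAmmo toggles between them.
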(event `self.ReceiveBeginPlay`
  (`parent.ReceiveBeginPlay`)
  (set `self.SnowValue` (`self.MaxSnowLoad`))
  (set `self.IceValue` (`self.MaxIceValue`)))

(event `IncreaseRate`
  ;[1 1 1] Spining
  (if (`KismetSystemLibrary.K2_IsValidTimerHandle` (`self.SlowDown_Handle`))
    (`KismetSystemLibrary.K2_ClearAndInvalidateTimerHandle` (`self.SlowDown_Handle`)))
  (set `self.Up` true)
  (bind _returnvalue (`KismetSystemLibrary.K2_SetTimer` null "AddSpeed" 0.1 true))
  (set `self.AddSpeed_Handle` _returnvalue))

(event `DecreaseRate`
  ;[1 1 1] Spining
  (if (`KismetSystemLibrary.K2_IsValidTimerHandle` (`self.AddSpeed_Handle`))
    (`KismetSystemLibrary.K2_ClearAndInvalidateTimerHandle` (`self.AddSpeed_Handle`)))
  (set `self.Up` false)
  (bind _returnvalue (`KismetSystemLibrary.K2_SetTimer` null "AddSpeed" 0.1 true))
  (set `self.SlowDown_Handle` _returnvalue))

(event `self.Spatula1.OnComponentBeginOverlap`
  (params (OverlappedComponent :type "PrimitiveComponent Object Reference") (OtherActor :type "Actor Object Reference") (OtherComp :type "PrimitiveComponent Object Reference") (OtherBodyIndex :type Integer) (bFromSweep :type Boolean) (SweepResult :type "HitResult Structure (by ref)"))
  (`self.ThrowSnowBall` (`self.Snow`)))

(event `self.Spatula3.OnComponentBeginOverlap`
  (params (OverlappedComponent :type "PrimitiveComponent Object Reference") (OtherActor :type "Actor Object Reference") (OtherComp :type "PrimitiveComponent Object Reference") (OtherBodyIndex :type Integer) (bFromSweep :type Boolean) (SweepResult :type "HitResult Structure (by ref)"))
  (`self.ThrowSnowBall` (`self.Snow`)))

(fn `AddSpeed`
  (locals (AddValue :type "Float (double-precision)" :default 10.0))
  (if (`self.Up`)
    (set `self.Rate` (+ (`self.Rate`) (`local.AddValue`)))
    (if (>= (`self.Rate`) 180.0)
      (set `self.Rate` 180.0))
    (else
      (set `self.Rate` (- (`self.Rate`) (`local.AddValue`)))
      (if (<= (`self.Rate`) 0.0)
        (set `self.Rate` 0.0)
        (`KismetSystemLibrary.K2_ClearAndInvalidateTimerHandle` (`self.SlowDown_Handle`)))))
  (set `RotatingMovementComponent.RotationRate` (`KismetMathLibrary.MakeRotator` (`self.Rate`)) (`self.RotatingMovement`)))

(fn `ChangeAmmo`
  (if (`self.Snow`)
    (set `self.Snow` false)
    (else
      (set `self.Snow` true))))

(fn `CheckSnowValue`
  (params (Snow :type Boolean))
  (returns (CanShoot :type Boolean))
  (if Snow
    (return (> (`self.SnowValue`) 0.0))
    (else
      (return (> (`self.IceValue`) 0.0)))))

(fn `ThrowSnowBall`
  (params (Snow :type Boolean))
  (bind _defaultsceneroot (`self.DefaultSceneRoot`))
  (bind (_returnvalue_roll _returnvalue_pitch _returnvalue_yaw) (`KismetMathLibrary.BreakRotator` (`SceneComponent.K2_GetComponentRotation` _defaultsceneroot)))
  (bind _canshoot (`self.CheckSnowValue` Snow))
  (if _canshoot
    (`|SpawnActorFromClass` (select `bool` Snow :`false` "/Game/SweetLove/Projectiles/BP_IceProjectile.BP_IceProjectile_C" :`true` "/Game/SweetLove/Projectiles/BP_SnowProjectile.BP_SnowProjectile_C" :!type "/Game/SweetLove/Projectiles/BP_SnowProjectile Class Reference") (`KismetMathLibrary.MakeTransform` (+ (`SceneComponent.K2_GetComponentLocation` _defaultsceneroot) (0.0 0.0 40.0)) (`KismetMathLibrary.MakeRotator` _returnvalue_roll _returnvalue_pitch (+ _returnvalue_yaw 90.0)) (0.2 0.2 0.2)) "AlwaysSpawn" "MultiplyWithRoot" null null)
    (if Snow
      (`/Engine/EditorBlueprintResources/StandardMacros.DecrementFloat` (`self.SnowValue`))
      (else
        (set `self.IceValue` (- (`self.IceValue`) 3.0))))))

(fn `UserConstructionScript`
  (`parent.UserConstructionScript`))