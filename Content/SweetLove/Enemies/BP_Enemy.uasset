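; BP_Enemy is an enemy actor that takes damage, drops an item and awards score when it dies.
; TakeDamage subtracts from HP and triggers the death event once HP reaches zero or below.
; On death, MakeDrop spawns a BP_Drop at the enemy's location, then the enemy sends its RewardScore to the player pawn and destroys itself.
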(event `Death_Event`
  (`self.MakeDrop`)
  (message `/Game/SweetLove/Interfaces/BPi_RecieveScore.RecieveScore` (`GameplayStatics.GetPlayerPawn` 0) (`self.RewardScore`))
  (`self.K2_DestroyActor`))

(fn `MakeDrop`
  (`|SpawnActorFromClass` "/Game/SweetLove/Enviroment/Drop/BP_Drop.BP_Drop_C" (`KismetMathLibrary.MakeTransform` (`SceneComponent.K2_GetComponentLocation` (`self.Scene`))) "AdjustIfPossibleButAlwaysSpawn" "MultiplyWithRoot" null null))

(fn `TakeDamage`
  (params (Value :type "Float (double-precision)"))
  (bind _output_get (set `self.HP` (- (`self.HP`) Value)))
  (if (<= _output_get 0.0)
    (`self.Death_Event`)))

(fn `UserConstructionScript`)