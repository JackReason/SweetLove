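; BP_Bomb is an exploding enemy that sets its own HP and score reward, then moves toward a target location via MoveToPool.
; PawnSensing diverts it to chase any seen pawn, and a retriggerable delay resumes the pool route one second after the last sighting.
; Any capsule overlap applies radial damage at the sweep location and destroys the bomb.
; Incoming damage events are forwarded to TakeDamage.
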(event `self.ReceiveBeginPlay`
  (set `self.RewardScore` 20)
  (set `self.HP` 40.0)
  (`self.MoveToPool`))

(event `MoveToPool`
  (`|AIMoveTo` self (`self.TargetLocation`) null 50.0))

(event `self.PawnSensing.OnSeePawn`
  (params (Pawn :type "Pawn Object Reference"))
  (`|ExecutionSequence`
    (:`then_0`
      (`|AIMoveTo` self (0.0 0.0 0.0) Pawn 30.0))
    (:`then_1`
      (`KismetSystemLibrary.RetriggerableDelay` 1.0)
      (`self.MoveToPool`))))

(event `/Game/SweetLove/Interfaces/BPi_RecieveDamage.RecieveDamage`
  (params (Value :type "Float (double-precision)"))
  (`self.TakeDamage` Value))

(event `self.CapsuleComponent.OnComponentBeginOverlap`
  (params (OverlappedComponent :type "PrimitiveComponent Object Reference") (OtherActor :type "Actor Object Reference") (OtherComp :type "PrimitiveComponent Object Reference") (OtherBodyIndex :type Integer) (bFromSweep :type Boolean) (SweepResult :type "HitResult Structure (by ref)"))
  (`GameplayStatics.ApplyRadialDamage` :`BaseDamage` 40.0 :`Origin` SweepResult_Location :`DamageRadius` 500.0 :`DamageCauser` self :`InstigatedByController` null)
  (`self.K2_DestroyActor`))

(fn `UserConstructionScript`)