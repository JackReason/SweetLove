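; BP_Demon is an enemy with health and a kill reward that heads for a pool location and attacks pawns it spots.
; A looping timer reissues the pool move, and reaching the pool triggers an attack plus self-damage.
; PawnSensing starts a chase, with a retriggerable delay returning it to the pool after sightings stop.
; Attacks rotate the capsule's yaw through a timeline, while box overlaps apply damage independently.
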(event `self.ReceiveBeginPlay`
  (set `self.RewardScore` 25)
  (set `self.HP` 65.0)
  (`self.MoveToPool`)
  (`KismetSystemLibrary.K2_SetTimerDelegate` (delegate `MoveToPool`) 8.0 true))

(event `MoveToPool`
  (`|AIMoveTo` self (`self.PoolLocation`) null 30.0
    (:`OnSuccess`
      (if (not (`self.AlreadyAttacking`))
        (`self.Attack_Event`)
        (`/Game/SweetLove/Interfaces/BPi_RecieveDamage.RecieveDamage` 30.0)))))

(event `self.PawnSensing.OnSeePawn`
  (params (Pawn :type "Pawn Object Reference"))
  (`|ExecutionSequence`
    (:`then_0`
      (`|AIMoveTo` self (0.0 0.0 0.0) Pawn 70.0
        (:`OnSuccess`
          (if (not (`self.AlreadyAttacking`))
            (`self.Attack_Event`)))))
    (:`then_1`
      (`KismetSystemLibrary.RetriggerableDelay` 1.0)
      (`self.MoveToPool`))))

(event `/Game/SweetLove/Interfaces/BPi_RecieveDamage.RecieveDamage`
  (params (Value :type "Float (double-precision)"))
  (`self.TakeDamage` Value))

(event `Attack_Event`
  (bind (_relativerotation_roll _relativerotation_pitch _relativerotation_yaw) (`KismetMathLibrary.BreakRotator` (`SceneComponent.RelativeRotation` (`self.CapsuleComponent`))))
  (set `self.AlreadyAttacking` true)
  (set `self.TempYaw` _relativerotation_yaw)
  (bind (_direction _newtrack_0) (`Timeline|RotateAttack` :!via `PlayFromStart`)
    (:`Update`
      (`SceneComponent.K2_SetRelativeRotation` (`self.CapsuleComponent`) (`KismetMathLibrary.MakeRotator` 0.0 0.0 (+ (`self.TempYaw`) _newtrack_0)) false false))
    (:`Finished`
      (set `self.AlreadyAttacking` false))))

(event `self.Box.OnComponentBeginOverlap`
  (params (OverlappedComponent :type "PrimitiveComponent Object Reference") (OtherActor :type "Actor Object Reference") (OtherComp :type "PrimitiveComponent Object Reference") (OtherBodyIndex :type Integer) (bFromSweep :type Boolean) (SweepResult :type "HitResult Structure (by ref)"))
  (`GameplayStatics.ApplyDamage` OtherActor 10.0))

(fn `UserConstructionScript`)