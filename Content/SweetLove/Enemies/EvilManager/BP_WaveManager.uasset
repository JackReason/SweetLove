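; Wave manager actor that spawns escalating waves of demons and occasional bombs at three random scene points, passing them a shared target location.
; Looping timers drive spawning and poll the enemy array for destroyed actors, updating the HUD count and wave number.
; A finished spawn batch enlarges the next wave, which starts after a pause once all enemies are gone.
; StopProducingWaves halts timers and signals game over to surviving enemies.
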(event `self.ReceiveBeginPlay`
  (bind _output_get (set `self.EnemiesPerWave` (`KismetMathLibrary.RandomIntegerInRange` 6 10)))
  (bind _output_get_2 (set `self.CurrentEnemiesCount` _output_get))
  (set `self.AliveEnemies` _output_get_2)
  (`KismetSystemLibrary.K2_SetTimerDelegate` (delegate `StartWave`) 1.0))

(event `StartWave`
  (bind _returnvalue (`KismetSystemLibrary.K2_SetTimer` null "SpawnEnemy" (`self.SpawnInterval`) true))
  (set `self.SpawnEnemy_handle` _returnvalue)
  (bind _returnvalue_2 (`KismetSystemLibrary.K2_SetTimer` null "CheckAliveEnemies" 0.5 true))
  (set `self.CheckAliveEnemies_Handle` _returnvalue_2)
  (`self.UpdateHud` (`self.AliveEnemies`)))

(event `EndWave`
  (bind _spawnenemy_handle (`self.SpawnEnemy_handle`))
  (if (`KismetSystemLibrary.K2_IsValidTimerHandle` _spawnenemy_handle)
    (`KismetSystemLibrary.K2_ClearAndInvalidateTimerHandle` _spawnenemy_handle)
    (`self.UpgradeWave`)))

(event `UpgradeWave`
  (`/Engine/EditorBlueprintResources/StandardMacros.IncrementInt` (`self.CurrentWave`)
    (:`  `
      (set `self.EnemiesPerWave` (+ (`self.EnemiesPerWave`) 2)))))

(event `PauseBetweenWaves`
  (`KismetSystemLibrary.K2_ClearAndInvalidateTimerHandle` (`self.CheckAliveEnemies_Handle`))
  (`KismetSystemLibrary.K2_SetTimer` null "CallNewWave" (`self.TimeBetweenWaves`)))

(event `/Game/SweetLove/Interfaces/BPi_RecieveTargetInfo.RecieveInfo`
  (params (TargetLocation :type "Vector Structure"))
  (set `self.TargetLocation` TargetLocation))

(event `/Game/SweetLove/Interfaces/BPi_StopWave.StopProducingWaves`
  (for _array_element (`self.EnemiesArray`)
    (`/Engine/EditorBlueprintResources/StandardMacros.IsValid` _array_element
      (:`Is Valid`
        (`/Game/SweetLove/Enemies/BP_Enemy.GameOver_Event` _array_element))))
  (`KismetSystemLibrary.K2_ClearAndInvalidateTimerHandle` (`self.CheckAliveEnemies_Handle`))
  (`KismetSystemLibrary.K2_ClearAndInvalidateTimerHandle` (`self.SpawnEnemy_handle`)))

(fn `CallNewWave`
  (`self.StartWave`)
  (bind _output_get (set `self.CurrentEnemiesCount` (`self.EnemiesPerWave`)))
  (bind _output_get_2 (set `self.AliveEnemies` _output_get))
  (`self.UpdateHud` _output_get_2))

(fn `CheckAliveEnemies`
  (bind _enemiesarray (`self.EnemiesArray`))
  (bind _returnvalue (`KismetArrayLibrary.Array_Length` (`self.EnemiesArray`)))
  (for _array_element _enemiesarray
    (`/Engine/EditorBlueprintResources/StandardMacros.IsValid` _array_element
      (:`Is Not Valid`
        (`KismetArrayLibrary.Array_RemoveItem` _enemiesarray _array_element)
        (set `self.AliveEnemies` (- (`self.AliveEnemies`) 1))
        (`self.UpdateHud` _returnvalue)
        (if (== _returnvalue 0)
          (`self.PauseBetweenWaves`))))))

(fn `SpawnEnemy`
  (bind _returnvalue (`SceneComponent.K2_GetComponentLocation` (select `int` (`KismetMathLibrary.RandomIntegerInRange` 0 2) :`0` (`self.Scene`) :`1` (`self.Scene1`) :`2` (`self.Scene2`))))
  (`/Engine/EditorBlueprintResources/StandardMacros.DecrementInt` (`self.CurrentEnemiesCount`)
    (:`  `
      (switch `int` (`KismetMathLibrary.RandomIntegerInRange` 0 4)
        (:`Default`
          (bind _returnvalue_2 (`|SpawnActorFromClass` "/Game/SweetLove/Enemies/BP_Demon.BP_Demon_C" (`KismetMathLibrary.MakeTransform` _returnvalue) "AlwaysSpawn" "MultiplyWithRoot" null (`self.TargetLocation`) null))
          (`KismetArrayLibrary.Array_Add` (`self.EnemiesArray`) _returnvalue_2)
          (if (<= (`self.CurrentEnemiesCount`) 0)
            (`self.EndWave`)))
        (:`0`
          (bind _returnvalue_3 (`|SpawnActorFromClass` "/Game/SweetLove/Enemies/BP_Bomb.BP_Bomb_C" (`KismetMathLibrary.MakeTransform` _returnvalue) "AlwaysSpawn" "MultiplyWithRoot" null (`self.TargetLocation`) null))
          (`KismetArrayLibrary.Array_Add` (`self.EnemiesArray`) _returnvalue_3)
          (if (<= (`self.CurrentEnemiesCount`) 0)
            (`self.EndWave`)))))))

(fn `UpdateHud`
  (params (Value :type Integer))
  (bind _asbp_hud (cast `/Game/SweetLove/GameBluePrints/BP_HUD` (`PlayerController.GetHUD` (`GameplayStatics.GetPlayerController` 0))))
  (`/Game/SweetLove/GameBluePrints/BP_HUD.ChangeEnemiesCountAndWave` _asbp_hud Value (`self.CurrentWave`)))

(fn `UserConstructionScript`)