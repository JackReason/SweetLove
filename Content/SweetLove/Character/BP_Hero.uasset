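; BP_Hero is the player character, spawning and attaching a BP_SnowThrower that fires snow or ice ammo.
; Enhanced Input drives movement, throwing, ammo switching and camera-trace aiming, while a timeline bobs the legs with random footstep sounds.
; A looping timer syncs ammo to BP_HUD and the belt's charge meshes.
; Damage raises stress, which decays over time and ends the game at its limit; the non-aim targeting timer is never wired.
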(event `self.ReceiveBeginPlay`
  (bind _weaponslot (`self.WeaponSlot`))
  (bind _asbp_hero_controller (cast `/Game/SweetLove/GameBluePrints/BP_HeroController` (`GameplayStatics.GetPlayerController` 0)))
  (bind _returnvalue (pcsubsystem `EnhancedInputLocalPlayerSubsystem` _asbp_hero_controller))
  (`/Engine/EditorBlueprintResources/StandardMacros.IsValid` _returnvalue
    (:`Is Valid`
      (`EnhancedInputSubsystemInterface.AddMappingContext` _returnvalue "/Game/SweetLove/Character/Controlls/IMS_Hero.IMS_Hero" 0 (struct))
      (bind _returnvalue_2 (`|SpawnActorFromClass` "/Game/SweetLove/Weapons/BP_SnowThrower.BP_SnowThrower_C" (`KismetMathLibrary.MakeTransform` (`SceneComponent.K2_GetComponentLocation` _weaponslot) (`KismetMathLibrary.MakeRotator` 0.0 0.0 270.0)) "AlwaysSpawn" "MultiplyWithRoot" null null))
      (bind _output_get (set `self.CurrentWeapon` _returnvalue_2))
      (`self.K2_AttachToComponent` _output_get _weaponslot "None" "SnapToTarget" "KeepWorld" "KeepWorld" false)
      (`KismetSystemLibrary.K2_SetTimer` null "CheckOnSnowValue" 2.0 true)
      (`self.RegenerateStress_Event`))))

(event `EnhancedInput|/Game/SweetLove/Character/Controlls/IA_See`
  (params (ActionValue :type "Vector2D Structure") (ElapsedSeconds :type "Float (double-precision)") (TriggeredSeconds :type "Float (double-precision)") (InputAction :type "InputAction Object Reference" :default "/Game/SweetLove/Character/Controlls/IA_See.IA_See"))
  ;[1 1 1] Mouse Control
  (:`Triggered`
    (`self.AddControllerYawInput` ActionValue_X)
    (`self.AddControllerPitchInput` (* ActionValue_Y -1.0))))

(event `EnhancedInput|/Game/SweetLove/Character/Controlls/IA_Walk`
  (params (ActionValue :type "Vector2D Structure") (ElapsedSeconds :type "Float (double-precision)") (TriggeredSeconds :type "Float (double-precision)") (InputAction :type "InputAction Object Reference" :default "/Game/SweetLove/Character/Controlls/IA_Walk.IA_Walk"))
  (bind (_returnvalue_roll _returnvalue_pitch _returnvalue_yaw) (`KismetMathLibrary.BreakRotator` (`self.GetControlRotation`)))
  (bind (_returnvalue_roll_2 _returnvalue_pitch_2 _returnvalue_yaw_2) (`KismetMathLibrary.BreakRotator` (`self.GetControlRotation`)))
  ;[1 1 1] Input
  (:`Triggered`
    (`self.AddMovementInput` (`KismetMathLibrary.GetRightVector` (`KismetMathLibrary.MakeRotator` _returnvalue_roll 0.0 _returnvalue_yaw)) ActionValue_X)
    (`self.AddMovementInput` (`KismetMathLibrary.GetForwardVector` (`KismetMathLibrary.MakeRotator` 0.0 0.0 _returnvalue_yaw_2)) ActionValue_Y))
  (:`Started`
    (`self.StartWalking`)
    (set `self.Go` true))
  (:`Completed`
    (set `self.Go` false)))

(event `EnhancedInput|/Game/SweetLove/Character/Controlls/IA_Throw`
  (params (ActionValue :type Boolean) (ElapsedSeconds :type "Float (double-precision)") (TriggeredSeconds :type "Float (double-precision)") (InputAction :type "InputAction Object Reference" :default "/Game/SweetLove/Character/Controlls/IA_Throw.IA_Throw"))
  (bind _currentweapon (`self.CurrentWeapon`))
  ;[1 1 1] Input
  (:`Started`
    (`/Game/SweetLove/Weapons/BP_SnowThrower.IncreaseRate` _currentweapon))
  (:`Completed`
    (`/Game/SweetLove/Weapons/BP_SnowThrower.DecreaseRate` _currentweapon)))

(event `EnhancedInput|/Game/SweetLove/Character/Controlls/IA_Aim`
  (params (ActionValue :type Boolean) (ElapsedSeconds :type "Float (double-precision)") (TriggeredSeconds :type "Float (double-precision)") (InputAction :type "InputAction Object Reference" :default "/Game/SweetLove/Character/Controlls/IA_Aim.IA_Aim"))
  (bind _aimball (`self.AimBall`))
  (bind _camera (`self.Camera`))
  (bind _returnvalue (`SceneComponent.K2_GetComponentLocation` _camera))
  ;[1 1 1] Input
  (:`Started`
    (`SceneComponent.SetVisibility` (`self.AimBall`) true false)
    (set `/Game/SweetLove/Weapons/BP_SnowThrower.Aiming` true (`self.CurrentWeapon`))
    (`KismetSystemLibrary.K2_PauseTimerHandle` (`self.SendingTargetToWeapon_Handle`)))
  (:`Ongoing`
    (bind _output_get (set `self.StartLocation` _returnvalue))
    (bind _output_get_2 (set `self.EndLocation` (+ _returnvalue (* (`KismetMathLibrary.GetForwardVector` (`SceneComponent.K2_GetComponentRotation` _camera)) 1500.0))))
    (bind (_outhit _returnvalue_2) (`KismetSystemLibrary.LineTraceSingle` :`Start` _output_get :`End` _output_get_2 :`TraceChannel` "TraceTypeQuery1" :`DrawTime` 1.0))
    (if _returnvalue_2
      (`SceneComponent.K2_SetWorldLocation` _aimball (`.Location` (`GameplayStatics.BreakHitResult` _outhit)) false false)
      (set `/Game/SweetLove/Weapons/BP_SnowThrower.EndProjectileLocation` (`.Location` (`GameplayStatics.BreakHitResult` _outhit)) (`self.CurrentWeapon`))
      (else
        (`SceneComponent.K2_SetWorldLocation` _aimball (`self.EndLocation`) false false)
        (set `/Game/SweetLove/Weapons/BP_SnowThrower.EndProjectileLocation` (`self.EndLocation`) (`self.CurrentWeapon`)))))
  (:`Canceled`
    (`SceneComponent.SetVisibility` (`self.AimBall`) false false)
    (set `/Game/SweetLove/Weapons/BP_SnowThrower.Aiming` false (`self.CurrentWeapon`))
    (`KismetSystemLibrary.K2_UnPauseTimerHandle` (`self.SendingTargetToWeapon_Handle`))))

(event `EnhancedInput|/Game/SweetLove/Character/Controlls/IA_ChangeAmmoType`
  (params (ActionValue :type Boolean) (ElapsedSeconds :type "Float (double-precision)") (TriggeredSeconds :type "Float (double-precision)") (InputAction :type "InputAction Object Reference" :default "/Game/SweetLove/Character/Controlls/IA_ChangeAmmoType.IA_ChangeAmmoType"))
  ;[1 1 1] Input
  (:`Completed`
    (`/Game/SweetLove/Weapons/BP_SnowThrower.ChangeAmmo` (`self.CurrentWeapon`))))

(event `StartWalking`
  (bind _leftleg (`self.LeftLeg`))
  (bind (_relativelocation_x _relativelocation_y _relativelocation_z) (`KismetMathLibrary.BreakVector` (`SceneComponent.RelativeLocation` (`self.RightLeg`))))
  (bind (_relativelocation_x_2 _relativelocation_y_2 _relativelocation_z_2) (`KismetMathLibrary.BreakVector` (`SceneComponent.RelativeLocation` _leftleg)))
  ;[1 1 1] Walking Animation
  (if (not (`self.AlreadyWalking`))
    (set `self.AlreadyWalking` true)
    (bind (_direction _zright) (`Timeline|Walking` :!via `PlayFromStart`)
      (:`Update`
        (`SceneComponent.K2_SetRelativeLocation` (`self.RightLeg`) (`KismetMathLibrary.MakeVector` _relativelocation_x _relativelocation_y (+ _relativelocation_z _zright)) false false)
        (`SceneComponent.K2_SetRelativeLocation` _leftleg (`KismetMathLibrary.MakeVector` _relativelocation_x_2 _relativelocation_y_2 (+ _relativelocation_z_2 (* _zright -1.0))) false false))
      (:`Finished`
        (`GameplayStatics.PlaySound2D` (select `int` (`KismetMathLibrary.RandomIntegerInRange` 0 3) :`0` "/Game/SweetLove/Sounds/SnowStep1_Cue.SnowStep1_Cue" :`1` "/Game/SweetLove/Sounds/SnowStep2_Cue.SnowStep2_Cue" :`2` "/Game/SweetLove/Sounds/SnowStep3_Cue.SnowStep3_Cue" :`3` "/Game/SweetLove/Sounds/SnowStep4_Cue.SnowStep4_Cue" :!type "SoundCue Object Reference") 1.0 1.0 0.0 null null)
        (set `self.AlreadyWalking` false)
        (if (`self.Go`)
          (`self.StartWalking`))))))

(event `/Game/SweetLove/Interfaces/BPi_RecieveIce.RecieveIce`
  (params (IceValue :type "Float (double-precision)"))
  ;[1 1 1] Add Ammo Ice
  (`self.TakeIceToBelt` IceValue))

(event `/Game/SweetLove/Interfaces/BPi_RecieveScore.RecieveScore`
  (params (Value :type Integer))
  ;[1 1 1] Scoring
  (bind _output_get (set `self.Score` (+ (`self.Score`) Value)))
  (bind _asbp_hud (cast `/Game/SweetLove/GameBluePrints/BP_HUD` (`PlayerController.GetHUD` (`GameplayStatics.GetPlayerController` 0))))
  (`/Game/SweetLove/GameBluePrints/BP_HUD.ChangeScore` _asbp_hud _output_get))

(event `self.ReceiveAnyDamage`
  (params (Damage :type "Float (single-precision)") (DamageType :type "DamageType Object Reference") (InstigatedBy :type "Controller Object Reference") (DamageCauser :type "Actor Object Reference"))
  ;[1 1 1] Damage to Hero
  (bind _output_get (set `self.Stress` (+ (`self.Stress`) Damage)))
  (bind _asbp_hud (cast `/Game/SweetLove/GameBluePrints/BP_HUD` (`PlayerController.GetHUD` (`GameplayStatics.GetPlayerController` 0))))
  (`/Game/SweetLove/GameBluePrints/BP_HUD.ChangeStress` _asbp_hud _output_get)
  ;[1 1 1] Game Over
  (if (>= (`self.Stress`) 100.0)
    (set `self.Stress` 0.0)
    (message `/Game/SweetLove/Interfaces/BPi_GameOverCall.GameOver` (`GameplayStatics.GetGameMode`) false)
    (`self.DisableInput` null)
    (`self.K2_DestroyActor` (`self.CurrentWeapon`))
    (`self.K2_DestroyActor`)))

(event `RegenerateStress_Event`
  ;[1 1 1] regenerate stress
  (`KismetSystemLibrary.K2_SetTimer` null "SubtractStress" 1.0 true))

(fn `CheckOnSnowValue`
  (locals (CurrentValue :type "Float (double-precision)") (MaxValue :type "Float (double-precision)") (CurrentValueInPercent :type "Float (double-precision)"))
  (bind _currentweapon (`self.CurrentWeapon`))
  (bind _currentvalueinpercent (`local.CurrentValueInPercent`))
  (bind _currentvalueinpercent_2 (`local.CurrentValueInPercent`))
  (bind _currentvalueinpercent_3 (`local.CurrentValueInPercent`))
  (bind _currentvalueinpercent_4 (`local.CurrentValueInPercent`))
  ;[1 1 1] To HUD
  (bind _asbp_hud (cast `/Game/SweetLove/GameBluePrints/BP_HUD` (`PlayerController.GetHUD` (`GameplayStatics.GetPlayerController` 0))))
  (`/Game/SweetLove/GameBluePrints/BP_HUD.ChangeSnowCharge` _asbp_hud (`/Game/SweetLove/Weapons/BP_SnowThrower.SnowValue` _currentweapon))
  (`/Game/SweetLove/GameBluePrints/BP_HUD.ChangeIceCharge` _asbp_hud (`/Game/SweetLove/Weapons/BP_SnowThrower.IceValue` _currentweapon))
  (if (`/Game/SweetLove/Weapons/BP_SnowThrower.Snow` _currentweapon)
    ;[1 1 1] SnowRelated
    (bind _output_get (set `local.CurrentValue` (`/Game/SweetLove/Weapons/BP_SnowThrower.SnowValue` _currentweapon)))
    (if (<= _output_get 0.0)
      (`SceneComponent.SetVisibility` (`self.Patron1`) false false)
      (`SceneComponent.SetVisibility` (`self.Patron2`) false false)
      (`SceneComponent.SetVisibility` (`self.Patron3`) false false)
      (`SceneComponent.SetVisibility` (`self.Patron4`) false false)
      (else
        (set `local.MaxValue` (`/Game/SweetLove/Weapons/BP_SnowThrower.MaxSnowLoad` (`self.CurrentWeapon`)))
        (set `local.CurrentValueInPercent` (* (/ (`local.CurrentValue`) (`local.MaxValue`)) 100.0))
        (if (and (<= _currentvalueinpercent_3 75.0) (> _currentvalueinpercent_3 50.0))
          (`SceneComponent.SetVisibility` (`self.Patron1`) false false)
          (`SceneComponent.SetVisibility` (`self.Patron2`) true false)
          (`SceneComponent.SetVisibility` (`self.Patron3`) true false)
          (`SceneComponent.SetVisibility` (`self.Patron4`) true false)
          (elif (and (<= _currentvalueinpercent_4 50.0) (> _currentvalueinpercent_4 25.0))
            (`SceneComponent.SetVisibility` (`self.Patron1`) false false)
            (`SceneComponent.SetVisibility` (`self.Patron2`) false false)
            (`SceneComponent.SetVisibility` (`self.Patron3`) true false)
            (`SceneComponent.SetVisibility` (`self.Patron4`) true false)
            (elif (<= (`local.CurrentValueInPercent`) 25.0)
              (`SceneComponent.SetVisibility` (`self.Patron1`) false false)
              (`SceneComponent.SetVisibility` (`self.Patron2`) false false)
              (`SceneComponent.SetVisibility` (`self.Patron3`) false false)
              (`SceneComponent.SetVisibility` (`self.Patron4`) true false))))))
    (else
      ;[1 1 1] Ice related
      (bind _output_get_2 (set `local.CurrentValue` (`/Game/SweetLove/Weapons/BP_SnowThrower.IceValue` (`self.CurrentWeapon`))))
      (if (<= _output_get_2 0.0)
        (`SceneComponent.SetVisibility` (`self.Ice1`) false false)
        (`SceneComponent.SetVisibility` (`self.Ice2`) false false)
        (`SceneComponent.SetVisibility` (`self.Ice3`) false false)
        (`SceneComponent.SetVisibility` (`self.Ice4`) false false)
        (else
          (set `local.MaxValue` (`/Game/SweetLove/Weapons/BP_SnowThrower.MaxIceValue` (`self.CurrentWeapon`)))
          (set `local.CurrentValueInPercent` (* (/ (`local.CurrentValue`) (`local.MaxValue`)) 100.0))
          (if (and (<= _currentvalueinpercent 75.0) (> _currentvalueinpercent 50.0))
            (`SceneComponent.SetVisibility` (`self.Ice1`) false false)
            (`SceneComponent.SetVisibility` (`self.Ice2`) true false)
            (`SceneComponent.SetVisibility` (`self.Ice3`) true false)
            (`SceneComponent.SetVisibility` (`self.Ice4`) true false)
            (elif (and (<= _currentvalueinpercent_2 50.0) (> _currentvalueinpercent_2 25.0))
              (`SceneComponent.SetVisibility` (`self.Ice1`) false false)
              (`SceneComponent.SetVisibility` (`self.Ice2`) false false)
              (`SceneComponent.SetVisibility` (`self.Ice3`) true false)
              (`SceneComponent.SetVisibility` (`self.Ice4`) true false)
              (elif (<= (`local.CurrentValueInPercent`) 25.0)
                (`SceneComponent.SetVisibility` (`self.Ice1`) false false)
                (`SceneComponent.SetVisibility` (`self.Ice2`) false false)
                (`SceneComponent.SetVisibility` (`self.Ice3`) false false)
                (`SceneComponent.SetVisibility` (`self.Ice4`) true false)
                (elif (> (`local.CurrentValueInPercent`) 75.0)
                  (`SceneComponent.SetVisibility` (`self.Ice1`) true false)
                  (`SceneComponent.SetVisibility` (`self.Ice2`) true false)
                  (`SceneComponent.SetVisibility` (`self.Ice3`) true false)
                  (`SceneComponent.SetVisibility` (`self.Ice4`) true false))))))))))

(fn `SendTargetToWeapon`
  (set `/Game/SweetLove/Weapons/BP_SnowThrower.EndProjectileLocation` (* (`SceneComponent.GetForwardVector` (`self.Body`)) 1000.0) (`self.CurrentWeapon`)))

(fn `SubtractStress`
  (bind _stress (`self.Stress`))
  (bind _result (`/Engine/EditorBlueprintResources/StandardMacros.DecrementFloat` _stress)
    (:`  `
      (bind _asbp_hud (cast `/Game/SweetLove/GameBluePrints/BP_HUD` (`PlayerController.GetHUD` (`GameplayStatics.GetPlayerController` 0))))
      (`/Game/SweetLove/GameBluePrints/BP_HUD.ChangeStress` _asbp_hud _result)
      (if (<= _stress 0.0)
        (set `self.Stress` 0.0)))))

(fn `TakeIceToBelt`
  (params (Value :type "Float (double-precision)"))
  (bind _currentweapon (`self.CurrentWeapon`))
  (bind _returnvalue (+ (`/Game/SweetLove/Weapons/BP_SnowThrower.IceValue` (`self.CurrentWeapon`)) Value))
  (if (>= _returnvalue 100.0)
    (bind _output_get (set `/Game/SweetLove/Weapons/BP_SnowThrower.IceValue` 100.0 _currentweapon))
    (bind _asbp_hud (cast `/Game/SweetLove/GameBluePrints/BP_HUD` (`PlayerController.GetHUD` (`GameplayStatics.GetPlayerController` 0))))
    (`/Game/SweetLove/GameBluePrints/BP_HUD.ChangeIceCharge` _asbp_hud _output_get)
    (else
      (bind _output_get_2 (set `/Game/SweetLove/Weapons/BP_SnowThrower.IceValue` _returnvalue _currentweapon))
      (bind _asbp_hud_2 (cast `/Game/SweetLove/GameBluePrints/BP_HUD` (`PlayerController.GetHUD` (`GameplayStatics.GetPlayerController` 0))))
      (`/Game/SweetLove/GameBluePrints/BP_HUD.ChangeIceCharge` _asbp_hud_2 _output_get_2))))

(fn `UserConstructionScript`)