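; BP_SnowProjectile is a snow projectile actor that damages what it hits and expires after a short lifespan.
; When its ProjectileMovement component activates, it applies the Blueprint's Velocity and Gravity variables to that component.
; A hit on the Sphere sends a fixed damage message to the other actor, spawns a splash effect, plays a 2D splash sound and destroys the projectile.
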(event `self.ReceiveBeginPlay`
  (`self.SetLifeSpan` 4.0))

(event `self.Sphere.OnComponentHit`
  (params (HitComponent :type "PrimitiveComponent Object Reference") (OtherActor :type "Actor Object Reference") (OtherComp :type "PrimitiveComponent Object Reference") (NormalImpulse :type "Vector Structure") (Hit :type "HitResult Structure (by ref)"))
  (message `/Game/SweetLove/Interfaces/BPi_RecieveDamage.RecieveDamage` OtherActor 30.0)
  (`NiagaraFunctionLibrary.SpawnSystemAtLocation` "/Game/SweetLove/FX/Splash_FX_Sysytem.Splash_FX_Sysytem" (`SceneComponent.K2_GetComponentLocation` (`self.Sphere`)))
  (`GameplayStatics.PlaySound2D` "/Game/SweetLove/Sounds/SnowSplash_Cue.SnowSplash_Cue" 1.0 1.0 0.0 null null)
  (`self.K2_DestroyActor`))

(event `self.ProjectileMovement.OnComponentActivated`
  (params (Component :type "ActorComponent Object Reference") (bReset :type Boolean))
  (bind _projectilemovement (`self.ProjectileMovement`))
  (set `MovementComponent.Velocity` (`self.Velocity`) _projectilemovement)
  (set `ProjectileMovementComponent.ProjectileGravityScale` (`self.Gravity`) _projectilemovement))

(fn `UserConstructionScript`)